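; Area trigger actor that ties a box volume to a multiplayer chat room identified by RoomID.
; On BeginPlay, a server with a local player controller joins or creates the room up front through MP_Chat_PlayerController.
; The local player's character joins or creates the room on entering the box, and on exit leaves it on both the controller and its ChatPanel.
; The room owner OnRep only prints a debug string.
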(event `self.ReceiveBeginPlay`
  (bind _returnvalue (`GameplayStatics.GetPlayerController` 0))
  ;[0.05 0.05 0.05] Skip if you don't want to create all rooms directly
  (if (`KismetSystemLibrary.IsServer`)
    (if (`Controller.IsLocalPlayerController` _returnvalue)
      (bind _asmp_chat_player_controller (cast `/MP_ChatSystem/Core/MP_Chat_PlayerController` _returnvalue))
      (`/MP_ChatSystem/Core/MP_Chat_PlayerController.Join Or Create Room` _asmp_chat_player_controller (`self.Room ID`) ""))))

(event `self.Box.OnComponentBeginOverlap`
  (params (OverlappedComponent :type "PrimitiveComponent Object Reference") (OtherActor :type "Actor Object Reference") (OtherComp :type "PrimitiveComponent Object Reference") (OtherBodyIndex :type Integer) (bFromSweep :type Boolean) (SweepResult :type "HitResult Structure (by ref)"))
  (bind _returnvalue (`GameplayStatics.GetPlayerController` 0))
  ;[0.05 0.05 0.05] Player Join Room(Enter BOX) or Leave Room(Exit BOX)
  (bind _ascharacter (cast `Character` OtherActor))
  (if (and (`Controller.IsLocalPlayerController` _returnvalue) (== _ascharacter (`GameplayStatics.GetPlayerCharacter` 0)))
    (bind _asmp_chat_player_controller (cast `/MP_ChatSystem/Core/MP_Chat_PlayerController` _returnvalue))
    (`/MP_ChatSystem/Core/MP_Chat_PlayerController.Join Or Create Room` _asmp_chat_player_controller (`self.Room ID`) "")))

(event `self.Box.OnComponentEndOverlap`
  (params (OverlappedComponent :type "PrimitiveComponent Object Reference") (OtherActor :type "Actor Object Reference") (OtherComp :type "PrimitiveComponent Object Reference") (OtherBodyIndex :type Integer))
  (bind _returnvalue (`GameplayStatics.GetPlayerController` 0))
  (bind _room_id (`self.Room ID`))
  ;[0.05 0.05 0.05] Player Join Room(Enter BOX) or Leave Room(Exit BOX)
  (bind _ascharacter (cast `Character` OtherActor))
  (if (and (`Controller.IsLocalPlayerController` _returnvalue) (== _ascharacter (`GameplayStatics.GetPlayerCharacter` 0)))
    (bind _asmp_chat_player_controller (cast `/MP_ChatSystem/Core/MP_Chat_PlayerController` _returnvalue))
    (`/MP_ChatSystem/Core/MP_Chat_PlayerController.Leave Chat Room` _asmp_chat_player_controller _room_id)
    (`/MP_ChatSystem/UI/MP_ChatPanel.Leave Chat Room` (`/MP_ChatSystem/Core/MP_Chat_PlayerController.Chat_Panel` _asmp_chat_player_controller) _room_id)))

(fn `OnRep_Room Owner`
  (`KismetSystemLibrary.PrintString` "Create"))

(fn `UserConstructionScript`)