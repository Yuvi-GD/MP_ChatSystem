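; Multiplayer chat room Blueprint that spawns a chat panel for the local player, shows the mouse cursor and relays messages to that panel.
; AddChatMessage runs on authority, appending to the Message array, updating the panel and printing the text.
; OnRep_Message pushes the newest entry to the panel on replication.
; Both paths tag messages with RoomID and take sender ID and name from player controller 0, not the stored message.
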(event `self.ReceiveBeginPlay`
  (bind _returnvalue (`GameplayStatics.GetPlayerController` 0))
  ;[0.05 0.05 0.05] UI Creation at Begin
  (if (`Controller.IsLocalPlayerController` _returnvalue)
    (bind _returnvalue_2 (`|CreateWidget` "/MP_ChatSystem/UI/MP_ChatPanel.MP_ChatPanel_C" null null))
    (bind _output_get (set `self.Chat UI` _returnvalue_2))
    (`UserWidget.AddToViewport` _output_get 0)
    (set `PlayerController.bShowMouseCursor` true _returnvalue)))

(event `Add Chat Message`
  (params (NewItem :type "String (by ref)"))
  (bind _returnvalue (`GameplayStatics.GetPlayerController` 0))
  ;[0.05 0.05 0.05] Add Chat Message
  (`/Engine/EditorBlueprintResources/ActorMacros.Switch Has Authority`
    (:`Authority`
      (`KismetArrayLibrary.Array_Add` (`self.Message`) NewItem)
      (bind _returnvalue_2 (message `MP_Chat_PlayerController_I.GetSenderID` _returnvalue))
      (bind _returnvalue_3 (message `MP_Chat_PlayerController_I.GetDisplayName` _returnvalue))
      (`/MP_ChatSystem/UI/MP_ChatPanel.OnMessageReceived_Event` (`self.Chat UI`) (`self.Room ID`) (make `MP_ChatMessage` _returnvalue_2 _returnvalue_3 NewItem))
      (`KismetSystemLibrary.PrintString` NewItem))))

(fn `OnRep_Message`
  (bind _returnvalue (`GameplayStatics.GetPlayerController` 0))
  (bind _message (`self.Message`))
  (bind _returnvalue_2 (message `MP_Chat_PlayerController_I.GetSenderID` _returnvalue))
  (bind _returnvalue_3 (message `MP_Chat_PlayerController_I.GetDisplayName` _returnvalue))
  (`/MP_ChatSystem/UI/MP_ChatPanel.OnMessageReceived_Event` (`self.Chat UI`) (`self.Room ID`) (make `MP_ChatMessage` _returnvalue_2 _returnvalue_3 (`|GetArrayItem` _message (`KismetArrayLibrary.Array_LastIndex` _message)))))

(fn `UserConstructionScript`)